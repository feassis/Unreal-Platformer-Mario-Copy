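; Mario-style warp pipe that carries the player to another location when they press Up or Down, depending on pipe orientation.
; Collision overlap opens a gate for the input, which then disables player control.
; Timelines slide the capsule into the pipe and out at WarpToLocal, rising or descending, with warp sounds, before restoring input.
; The construction script stacks instanced body segments to match the PipeEndPoint length.
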(event OnComponentBeginOverlap(Collision)
  (params (OverlappedComponent :type Primitive%20Component%20Object%20Reference) (OtherActor :type Actor%20Object%20Reference) (OtherComp :type Primitive%20Component%20Object%20Reference) (OtherBodyIndex :type Integer) (bFromSweep :type Boolean) (SweepResult :type Hit%20Result%20Structure%20%28by%20ref%29))
  (bind _warpinpoint (Variables|Default|GetWarpInPoint))
  (bind _warptolocal (Variables|Default|GetWarpToLocal))
  (bind _warpinpoint_2 (Variables|Default|GetWarpInPoint))
  (bind _warptolocal_2 (Variables|Default|GetWarpToLocal))
  (bind _returnvalue (Transformation|GetWorldLocation _warpinpoint))
  (bind (_x _y _z) (Math|Vector|BreakVector _warptolocal_2))
  (bind (_x_2 _y_2 _z_2) (Math|Vector|BreakVector _warptolocal))
  (bind _returnvalue_2 (Transformation|GetWorldLocation _warpinpoint_2))
  (bind (_x_3 _y_3 _z_3) (Math|Vector|BreakVector _returnvalue_2))
  (bind (_x_4 _y_4 _z_4) (Math|Vector|BreakVector _returnvalue))
  (bind _asbp_third_person_character (Utilities|Casting|CastToBP_ThirdPersonCharacter OtherActor))
  (Utilities|FlowControl|Gate true) ; enters at Open
)

(event OnComponentEndOverlap(Collision)
  (params (OverlappedComponent :type Primitive%20Component%20Object%20Reference) (OtherActor :type Actor%20Object%20Reference) (OtherComp :type Primitive%20Component%20Object%20Reference) (OtherBodyIndex :type Integer))
  (bind _warpinpoint (Variables|Default|GetWarpInPoint))
  (bind _warptolocal (Variables|Default|GetWarpToLocal))
  (bind _warpinpoint_2 (Variables|Default|GetWarpInPoint))
  (bind _warptolocal_2 (Variables|Default|GetWarpToLocal))
  (bind _returnvalue (Transformation|GetWorldLocation _warpinpoint))
  (bind (_x _y _z) (Math|Vector|BreakVector _warptolocal_2))
  (bind (_x_2 _y_2 _z_2) (Math|Vector|BreakVector _warptolocal))
  (bind _returnvalue_2 (Transformation|GetWorldLocation _warpinpoint_2))
  (bind (_x_3 _y_3 _z_3) (Math|Vector|BreakVector _returnvalue_2))
  (bind (_x_4 _y_4 _z_4) (Math|Vector|BreakVector _returnvalue))
  (Utilities|Casting|CastToBP_ThirdPersonCharacter OtherActor)
  (Utilities|FlowControl|Gate true) ; enters at Close
)

(event Input|EnhancedActionEvents|EnhancedInputActionIA_PlayerUP
  (params (ActionValue :type Boolean) (ElapsedSeconds :type Float%20%28double-precision%29) (TriggeredSeconds :type Float%20%28double-precision%29) (InputAction :type Input%20Action%20Object%20Reference :default "/Game/ThirdPerson/Input/Actions/IA_PlayerUP.IA_PlayerUP"))
  (bind _warpinpoint (Variables|Default|GetWarpInPoint))
  (bind _warptolocal (Variables|Default|GetWarpToLocal))
  (bind _warpinpoint_2 (Variables|Default|GetWarpInPoint))
  (bind _warptolocal_2 (Variables|Default|GetWarpToLocal))
  (bind _returnvalue (Transformation|GetWorldLocation _warpinpoint))
  (bind (_x _y _z) (Math|Vector|BreakVector _warptolocal_2))
  (bind (_x_2 _y_2 _z_2) (Math|Vector|BreakVector _warptolocal))
  (bind _returnvalue_2 (Transformation|GetWorldLocation _warpinpoint_2))
  (bind (_x_3 _y_3 _z_3) (Math|Vector|BreakVector _returnvalue_2))
  (bind (_x_4 _y_4 _z_4) (Math|Vector|BreakVector _returnvalue))
  (:Started
    (if (and (Variables|Default|GetCanInteract) (not (Variables|Default|GetIsDownPipe)))
      (Utilities|FlowControl|Gate true
        (:Exit
          (bind _output_get (Variables|Default|SetMyPlayer (stale OnComponentBeginOverlap(Collision) _asbp_third_person_character)))
          (Input|DisableInput _output_get (Game|GetPlayerController 0))
          (if (Variables|Default|GetIsDownPipe)
            (Utilities|FlowControl|Sequence
              (:then_0
                ;[0 0 0] EnterDown Pipe
                (bind _movement (Timeline|IntoDownPipe PlayFromStart)
                  (:Update
                    (Transformation|SetRelativeLocationAndRotation (Variables|/Script/Engine.Character|GetCapsuleComponent (Variables|Default|GetMyPlayer)) (Math|Vector|MakeVector _x_3 _y_3 (+ _movement _z_3)) "0, 0, 0" false false))
                  (:Finished
                    ;[0 0 0] Wair a bit before exiting out o pipe
                    (Utilities|FlowControl|Delay 0.4 :!label _label)
                    (Audio|PlaySound2D "/Game/Platformer/Audio/Mario_Warp.Mario_Warp" 1.0 1.0 0.0 0 0)
                    (if (Variables|Default|GetExitsRisingUp)
                      ;[0 0 0] Exit Rising UP Pipe
                      (bind _movement_2 (Timeline|Timeline PlayFromStart)
                        (:Update
                          (Transformation|SetRelativeLocationAndRotation (Variables|/Script/Engine.Character|GetCapsuleComponent (Variables|Default|GetMyPlayer)) (Math|Vector|MakeVector _x_2 _y_2 (+ _movement_2 _z_2)) "0, 0, 0" false false))
                        (:Finished
                          ;[0 0 0] Enable User Control
                          (Input|EnableInput (Game|GetPlayerCharacter 0) (Game|GetPlayerController 0) :!label _label_2)))
                      (else
                        ;[0 0 0] Exit Down Pipe
                        (bind _movement_3 (Timeline|Timeline_1 PlayFromStart)
                          (:Update
                            (Transformation|SetRelativeLocationAndRotation (Variables|/Script/Engine.Character|GetCapsuleComponent (Variables|Default|GetMyPlayer)) (Math|Vector|MakeVector _x _y (+ _movement_3 _z)) "0, 0, 0" false false))
                          (:Finished
                            (goto _label_2))))))))
              (:then_1
                ;[0 0 0] Warp SFX
                (Utilities|FlowControl|Delay 0.2 :!label _label_3)
                (Audio|PlaySound2D "/Game/Platformer/Audio/Mario_Warp.Mario_Warp" 1.0 1.0 0.0 0 0)))
            (else
              (Utilities|FlowControl|Sequence
                (:then_0
                  (goto _label_3))
                (:then_1
                  ;[0 0 0] Enter Rising UP Pipe
                  (bind _movement_4 (Timeline|Timeline_0 PlayFromStart)
                    (:Update
                      (Transformation|SetRelativeLocationAndRotation (Variables|/Script/Engine.Character|GetCapsuleComponent (Variables|Default|GetMyPlayer)) (Math|Vector|MakeVector _x_4 _y_4 (+ _movement_4 _z_4)) "0, 0, 0" false false))
                    (:Finished
                      (goto _label))))))))))))

(event Input|EnhancedActionEvents|EnhancedInputActionIA_PlayerDown
  (params (ActionValue :type Boolean) (ElapsedSeconds :type Float%20%28double-precision%29) (TriggeredSeconds :type Float%20%28double-precision%29) (InputAction :type Input%20Action%20Object%20Reference :default "/Game/ThirdPerson/Input/Actions/IA_PlayerDown.IA_PlayerDown"))
  (bind _warpinpoint (Variables|Default|GetWarpInPoint))
  (bind _warptolocal (Variables|Default|GetWarpToLocal))
  (bind _warpinpoint_2 (Variables|Default|GetWarpInPoint))
  (bind _warptolocal_2 (Variables|Default|GetWarpToLocal))
  (bind _returnvalue (Transformation|GetWorldLocation _warpinpoint))
  (bind (_x _y _z) (Math|Vector|BreakVector _warptolocal_2))
  (bind (_x_2 _y_2 _z_2) (Math|Vector|BreakVector _warptolocal))
  (bind _returnvalue_2 (Transformation|GetWorldLocation _warpinpoint_2))
  (bind (_x_3 _y_3 _z_3) (Math|Vector|BreakVector _returnvalue_2))
  (bind (_x_4 _y_4 _z_4) (Math|Vector|BreakVector _returnvalue))
  (:Started
    (if (and (Variables|Default|GetCanInteract) (Variables|Default|GetIsDownPipe))
      (Utilities|FlowControl|Gate true
        (:Exit
          (bind _output_get (Variables|Default|SetMyPlayer (stale OnComponentBeginOverlap(Collision) _asbp_third_person_character)))
          (Input|DisableInput _output_get (Game|GetPlayerController 0))
          (if (Variables|Default|GetIsDownPipe)
            (Utilities|FlowControl|Sequence
              (:then_0
                ;[0 0 0] EnterDown Pipe
                (bind _movement (Timeline|IntoDownPipe PlayFromStart)
                  (:Update
                    (Transformation|SetRelativeLocationAndRotation (Variables|/Script/Engine.Character|GetCapsuleComponent (Variables|Default|GetMyPlayer)) (Math|Vector|MakeVector _x_3 _y_3 (+ _movement _z_3)) "0, 0, 0" false false))
                  (:Finished
                    ;[0 0 0] Wair a bit before exiting out o pipe
                    (Utilities|FlowControl|Delay 0.4 :!label _label)
                    (Audio|PlaySound2D "/Game/Platformer/Audio/Mario_Warp.Mario_Warp" 1.0 1.0 0.0 0 0)
                    (if (Variables|Default|GetExitsRisingUp)
                      ;[0 0 0] Exit Rising UP Pipe
                      (bind _movement_2 (Timeline|Timeline PlayFromStart)
                        (:Update
                          (Transformation|SetRelativeLocationAndRotation (Variables|/Script/Engine.Character|GetCapsuleComponent (Variables|Default|GetMyPlayer)) (Math|Vector|MakeVector _x_2 _y_2 (+ _movement_2 _z_2)) "0, 0, 0" false false))
                        (:Finished
                          ;[0 0 0] Enable User Control
                          (Input|EnableInput (Game|GetPlayerCharacter 0) (Game|GetPlayerController 0) :!label _label_2)))
                      (else
                        ;[0 0 0] Exit Down Pipe
                        (bind _movement_3 (Timeline|Timeline_1 PlayFromStart)
                          (:Update
                            (Transformation|SetRelativeLocationAndRotation (Variables|/Script/Engine.Character|GetCapsuleComponent (Variables|Default|GetMyPlayer)) (Math|Vector|MakeVector _x _y (+ _movement_3 _z)) "0, 0, 0" false false))
                          (:Finished
                            (goto _label_2))))))))
              (:then_1
                ;[0 0 0] Warp SFX
                (Utilities|FlowControl|Delay 0.2 :!label _label_3)
                (Audio|PlaySound2D "/Game/Platformer/Audio/Mario_Warp.Mario_Warp" 1.0 1.0 0.0 0 0)))
            (else
              (Utilities|FlowControl|Sequence
                (:then_0
                  (goto _label_3))
                (:then_1
                  ;[0 0 0] Enter Rising UP Pipe
                  (bind _movement_4 (Timeline|Timeline_0 PlayFromStart)
                    (:Update
                      (Transformation|SetRelativeLocationAndRotation (Variables|/Script/Engine.Character|GetCapsuleComponent (Variables|Default|GetMyPlayer)) (Math|Vector|MakeVector _x_4 _y_4 (+ _movement_4 _z_4)) "0, 0, 0" false false))
                    (:Finished
                      (goto _label))))))))))))

(fn ConstructionScript
  (for _index (range 0 (Math|Float|Truncate (/ (Math|Vector|VectorLength (Variables|Default|GetPipeEndPoint)) 1e+02)))
    (Components|InstancedStaticMesh|AddInstance (Variables|Default|GetPipeBody) (Math|Transform|MakeTransform (Math|Vector|MakeVector 0.0 0.0 (* _index -1e+02))) false)))