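; BP_LevelSettings runs a platformer level's music, countdown timer and completion sequence.
; On begin play and respawn it resets the controller's timer, starts music and binds game mode, character and end-flag events.
; A looping timer counts down, plays a low-time warning, speeds up music and kills the player at zero.
; Completion converts remaining time to points, saves coins, points and lives to the GameInstance, then opens the next level.
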(event Custom|PlayerRespawned
  (Utilities|FlowControl|Sequence
    (:then_0
      ;[0 0 0] Listens out for player respawned
      (bind _asbp_third_person_game_mode (Utilities|Casting|CastToBP_ThirdPersonGameMode (Game|GetGameMode)))
      (EventDispatchers|AssignPlayerRespawned _asbp_third_person_game_mode (delegate Custom|PlayerRespawned_Event)))
    (:then_1
      ;[0 0 0] Ref to player controller and set timer variable
      (bind _asbp_player_controller (Utilities|Casting|CastToBP_PlayerController (Game|GetPlayerController 0)))
      (bind _output_get (Variables|Default|SetPlayerControllerRef _asbp_player_controller))
      (bind _output_get_2 (Variables|/Game/Platformer/Blueprints/Framework/BP_PlayerController.BP_PlayerController_C|SetTimer _output_get (Variables|Default|GetTimeLimitMax)))
      (Variables|Default|SetTimeLimitCurrent _output_get_2))
    (:then_2
      ;[0 0 0] Sets Level Music
      (Audio|Components|Audio|SetSound (Variables|Default|GetLevel%20Music) (Variables|Default|GetLevelMusicChoice))
      (Utilities|FlowControl|Delay 0.75)
      (Audio|Components|Audio|Play (Variables|Default|GetLevel%20Music) 0.0))
    (:then_3
      ;[0 0 0] Run TImer and Playe Apropriate music
      (Utilities|FlowControl|RetriggerableDelay 1.0)
      (bind _returnvalue (Utilities|Time|SetTimerbyEvent (delegate Custom|RunLevelTimer) (Variables|Default|GetTimePlayRate) true))
      (bind _output_get_3 (Variables|Default|SetLevelTimer _returnvalue)))
    (:then_4
      ;[0 0 0] Stop Any music if player dies
      (bind _asbp_third_person_character (Utilities|Casting|CastToBP_ThirdPersonCharacter (Game|GetPlayerCharacter 0)))
      (EventDispatchers|AssignPlayerStartsDeathSequence _asbp_third_person_character (delegate Custom|PlayerStartsDeathSequence_Event)))
    (:then_5
      (EventDispatchers|AssignLevelComplete (Variables|Default|GetEndOfLevelFlag) (delegate Custom|LevelComplete_Event)))))

(event Custom|PlayerRespawned_Event
  ;[0 0 0] Listens out for player respawned
  (Audio|Components|Audio|SetPitchMultiplier (Variables|Default|GetLevel%20Music) 1.0)
  (CallFunction|PlayerRespawned))

(event Custom|RunLevelTimer
  (bind _level_music (Variables|Default|GetLevel%20Music))
  (bind _timelimitcurrent (Variables|Default|GetTimeLimitCurrent))
  ;[0 0 0] Run TImer and Playe Apropriate music
  (if (== _timelimitcurrent 0)
    (Utilities|Time|ClearandInvalidateTimerbyHandle (stale Custom|PlayerRespawned _output_get_3))
    (Audio|Components|Audio|Stop (Variables|Default|GetLevel%20Music))
    (Audio|Components|Audio|Stop (Variables|Default|GetTimeRunningOutWarning))
    (bind _asbp_third_person_character (Utilities|Casting|CastToBP_ThirdPersonCharacter (Game|GetPlayerCharacter 0)))
    (Default|PlayerDies _asbp_third_person_character)
    (else
      (bind _result (Math|Integer|DecrementInt _timelimitcurrent)
        (:%20%20
          (Variables|/Game/Platformer/Blueprints/Framework/BP_PlayerController.BP_PlayerController_C|SetTimer (Variables|Default|GetPlayerControllerRef) _result)
          (if (== _timelimitcurrent (Variables|Default|GetTimeRunningOut))
            (Class|AudioComponent|SetPaused (Variables|Default|GetLevel%20Music) true)
            (Audio|Components|Audio|Play (Variables|Default|GetTimeRunningOutWarning) 0.0)
            (Utilities|FlowControl|Delay 2.8)
            (Class|AudioComponent|SetPaused _level_music false)
            (Audio|Components|Audio|SetPitchMultiplier _level_music 1.05)))))))

(event Custom|PlayerStartsDeathSequence_Event
  ;[0 0 0] Stop Any music if player dies
  (Audio|Components|Audio|Stop (Variables|Default|GetLevel%20Music))
  (Utilities|Time|ClearandInvalidateTimerbyHandle (Variables|Default|GetLevelTimer)))

(event Custom|LevelComplete_Event
  (bind _returnvalue (Game|GetPlayerController 0))
  (bind _returnvalue_2 (Game|GetGameInstance))
  (bind _asbp_player_controller (Utilities|Casting|CastToBP_PlayerController _returnvalue))
  (bind _asbp_game_instance (Utilities|Casting|CastToBP_GameInstance _returnvalue_2))
  (Audio|Components|Audio|Stop (Variables|Default|GetLevel%20Music))
  (Utilities|Time|PauseTimerbyHandle (Variables|Default|GetLevelTimer))
  (Utilities|FlowControl|Delay 3.0)
  (Components|Activation|Activate (Variables|Default|GetLevelComplete) false)
  ;[0 0 0] Decrementing Time remaing on level compete and reward points
  (Utilities|FlowControl|Delay 0.05 :!label _label)
  (bind _result (Math|Integer|DecrementInt (Variables|/Game/Platformer/Blueprints/Framework/BP_PlayerController.BP_PlayerController_C|GetTimer (Variables|Default|GetPlayerControllerRef)))
    (:%20%20
      (if (> _result 0)
        (Default|AddPoints (Variables|Default|GetPlayerControllerRef) 50)
        (Audio|PlaySound2D "/Engine/VREditor/Sounds/UI/Camera_Shutter.Camera_Shutter" 1.0 1.0 0.0 0 0)
        (goto _label)
        (else
          (Variables|/Game/Platformer/Blueprints/Framework/BP_GameInstance.BP_GameInstance_C|SetCoins _asbp_game_instance (Variables|/Game/Platformer/Blueprints/Framework/BP_PlayerController.BP_PlayerController_C|GetCoins _asbp_player_controller))
          (Variables|/Game/Platformer/Blueprints/Framework/BP_GameInstance.BP_GameInstance_C|SetPoints _asbp_game_instance (Variables|/Game/Platformer/Blueprints/Framework/BP_PlayerController.BP_PlayerController_C|GetPoints _asbp_player_controller))
          (Variables|/Game/Platformer/Blueprints/Framework/BP_GameInstance.BP_GameInstance_C|SetLives _asbp_game_instance (Variables|/Game/Platformer/Blueprints/Framework/BP_PlayerController.BP_PlayerController_C|GetLives _asbp_player_controller))
          (Utilities|FlowControl|Delay 2.0)
          (Game|OpenLevel(byName) (Variables|Default|GetLevelToGoTo)))))))

(event EventBeginPlay
  (Utilities|FlowControl|Sequence
    (:then_0
      ;[0 0 0] Listens out for player respawned
      (bind _asbp_third_person_game_mode (Utilities|Casting|CastToBP_ThirdPersonGameMode (Game|GetGameMode)))
      (EventDispatchers|AssignPlayerRespawned _asbp_third_person_game_mode (delegate Custom|PlayerRespawned_Event)))
    (:then_1
      ;[0 0 0] Ref to player controller and set timer variable
      (bind _asbp_player_controller (Utilities|Casting|CastToBP_PlayerController (Game|GetPlayerController 0)))
      (bind _output_get (Variables|Default|SetPlayerControllerRef _asbp_player_controller))
      (bind _output_get_2 (Variables|/Game/Platformer/Blueprints/Framework/BP_PlayerController.BP_PlayerController_C|SetTimer _output_get (Variables|Default|GetTimeLimitMax)))
      (Variables|Default|SetTimeLimitCurrent _output_get_2))
    (:then_2
      ;[0 0 0] Sets Level Music
      (Audio|Components|Audio|SetSound (Variables|Default|GetLevel%20Music) (Variables|Default|GetLevelMusicChoice))
      (Utilities|FlowControl|Delay 0.75)
      (Audio|Components|Audio|Play (Variables|Default|GetLevel%20Music) 0.0))
    (:then_3
      ;[0 0 0] Run TImer and Playe Apropriate music
      (Utilities|FlowControl|RetriggerableDelay 1.0)
      (bind _returnvalue (Utilities|Time|SetTimerbyEvent (delegate Custom|RunLevelTimer) (Variables|Default|GetTimePlayRate) true))
      (bind _output_get_3 (Variables|Default|SetLevelTimer _returnvalue)))
    (:then_4
      ;[0 0 0] Stop Any music if player dies
      (bind _asbp_third_person_character (Utilities|Casting|CastToBP_ThirdPersonCharacter (Game|GetPlayerCharacter 0)))
      (EventDispatchers|AssignPlayerStartsDeathSequence _asbp_third_person_character (delegate Custom|PlayerStartsDeathSequence_Event)))
    (:then_5
      (EventDispatchers|AssignLevelComplete (Variables|Default|GetEndOfLevelFlag) (delegate Custom|LevelComplete_Event)))))

(fn ConstructionScript)