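; Bouncing fireball projectile for the platformer, driven entirely by its ProjectileMovement bounce event.
; Hitting a wall or steep slope, judged by the absolute Z of the impact normal, makes it explode immediately.
; Near-horizontal floors and ceilings let it bounce, incrementing a counter until BounceLimit triggers the same explosion.
; The explosion spawns a particle effect with attached sound, then destroys the actor.
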(event OnProjectileBounce(ProjectileMovement)
  (params (ImpactResult :type Hit%20Result%20Structure%20%28by%20ref%29) (ImpactVelocity :type Vector%20%28by%20ref%29 :default "0, 0, 0"))
  (if (< (.Z (Math|Vector|BreakVector (Math|Vector|VectorGetAbs (.Normal (Collision|BreakHitResult ImpactResult))))) 0.9)
    (bind _returnvalue (Effects|SpawnEmitteratLocation "/Game/StarterContent/Particles/P_Explosion.P_Explosion" (Transformation|GetWorldLocation (Variables|Default|GetSphere)) :!label _label))
    (Audio|SpawnSoundAttached "/Game/StarterContent/Audio/Explosion_Cue.Explosion_Cue" _returnvalue "None" "0, 0, 0" "0, 0, 0" "KeepRelativeOffset" false 1.0 1.0 0.0 0 0)
    (Actor|DestroyActor)
    (else
      (bind _result (Math|Integer|IncrementInt (Variables|Default|GetFireballBounceCounter))
        (:%20%20
          (if (>= _result (Variables|Default|GetBounceLimit))
            (goto _label)))))))

(event EventBeginPlay)

(event Collision|EventActorBeginOverlap
  (params (OtherActor :type Actor%20Object%20Reference)))

(event EventTick
  (params (DeltaSeconds :type Float%20%28single-precision%29)))

(fn ConstructionScript)