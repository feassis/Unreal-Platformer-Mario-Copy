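; BP_Points is a short-lived floating score popup that displays a point amount through a WBP_Points widget component.
; On BeginPlay it casts the widget, sets its text from PointsToAdd and plays the widget's PointsAnimation.
; It waits for the animation's end time, then destroys itself.
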(event EventBeginPlay
  (bind _aswbp_points (Utilities|Casting|CastToWBP_Points (UserInterface|GetWidget (Variables|Default|GetWidget))))
  (UserInterface|Animation|PlayAnimation _aswbp_points (Variables|/Game/Platformer/UI/WBP_Points.WBP_Points_C|GetPoints_Animation _aswbp_points) 0.0 1 "Forward" 1.0 false)
  (Variables|/Script/UMG.TextBlock|SetText (Variables|/Game/Platformer/UI/WBP_Points.WBP_Points_C|GetText_Points _aswbp_points) (Utilities|Text|ToText(Integer) (Variables|Default|GetPointsToAdd)))
  (Utilities|FlowControl|Delay (Class|WidgetAnimation|GetEndTime (Variables|/Game/Platformer/UI/WBP_Points.WBP_Points_C|GetPoints_Animation _aswbp_points)))
  (Actor|DestroyActor))

(fn ConstructionScript)