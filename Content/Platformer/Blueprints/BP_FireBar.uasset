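; BP_FireBar is a rotating fire bar for the platformer, made of a line of flame balls.
; The construction script stacks a configurable number of evenly spaced, scaled flame balls along local Z as instances of one InstancedStaticMesh.
; It resizes and centers a Box component over the bar's length and passes the rotation rate to RotatingMovement.
; The event graph holds no active logic, so overlaps trigger nothing here.
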(event EventBeginPlay)

(event Collision|EventActorBeginOverlap
  (params (OtherActor :type Actor%20Object%20Reference)))

(event EventTick
  (params (DeltaSeconds :type Float%20%28single-precision%29)))

(fn ConstructionScript
  (bind _flameballdistanceapart (Variables|BarCustomization|GetFlameBallDistanceApart))
  (bind _box (Variables|Default|GetBox))
  (for _index (range 0 (- (Variables|BarCustomization|GetFlameBalNumber) 1))
    (Utilities|FlowControl|Sequence
      (:then_0
        ;[0 0 0] Add Instances of Flame Ball
        (Components|InstancedStaticMesh|AddInstance (Variables|Default|GetInstancedStaticMesh) (Math|Transform|MakeTransform (Math|Vector|MakeVector 0.0 0.0 (Math|Conversions|ToFloat(Integer) (* _index _flameballdistanceapart))) "0, 0, 0" (Variables|BarCustomization|GetFlameBallSize)) false))
      (:then_1
        ;[0 0 0] Box Extend Size
        (Components|Box|SetBoxExtent _box (Math|Vector|MakeVector 1e+01 5e+01 (Math|Conversions|ToFloat(Integer) (/ (* (+ _index 1) _flameballdistanceapart) 2))) true)
        (Transformation|SetRelativeLocation _box (Math|Vector|MakeVector 0.0 0.0 (Math|Conversions|ToFloat(Integer) (/ (* (+ _index 1) _flameballdistanceapart) 2))) false false))
      (:then_2
        ;[0 0 0] Set Rotation Rate
        (Variables|/Script/Engine.RotatingMovementComponent|SetRotationRate (Variables|Default|GetRotatingMovement) (Variables|BarCustomization|GetRotationRate))))))