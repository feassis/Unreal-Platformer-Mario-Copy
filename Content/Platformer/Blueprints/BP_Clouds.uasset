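; BP_Clouds is a scenery actor that scatters cloud mesh instances inside an adjustable box volume.
; The Construction Script sizes the SpawnArea box from the extent variables, then adds instances to the Clouds instanced mesh component at random points within it.
; Each instance gets zero rotation and a random uniform scale, with no seed, so the layout changes whenever construction reruns.
; The Event Graph holds no runtime logic.
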(event EventBeginPlay)

(event Collision|EventActorBeginOverlap
  (params (OtherActor :type Actor%20Object%20Reference)))

(event EventTick
  (params (DeltaSeconds :type Float%20%28single-precision%29)))

(fn ConstructionScript
  (bind _spawnarea (Variables|Default|GetSpawnArea))
  (Components|Box|SetBoxExtent (Variables|Default|GetSpawnArea) (Math|Vector|MakeVector (Variables|Default|GetSpawnExtentX) (Variables|Default|GetSpawnExtentY) (Variables|Default|GetSpawnExtentZ)) true)
  (for _index (range 0 (Variables|Default|GetInsancesToSpawn))
    (Components|InstancedStaticMesh|AddInstance (Variables|Default|GetClouds) (Math|Transform|MakeTransform (Math|Random|RandomPointinBoundingBox (Variables|/Script/Engine.SceneComponent|GetRelativeLocation _spawnarea) (Components|Box|GetScaledBoxExtent _spawnarea)) "0, 0, 0" (Math|Conversions|ToVector(Float) (Math|Random|RandomFloatinRange (Variables|Default|GetScaleMIn) (Variables|Default|GetScaleMax)))) false)))