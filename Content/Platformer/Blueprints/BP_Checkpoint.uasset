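; BP_Checkpoint is a platformer checkpoint that updates the respawn point when the player character overlaps its box.
; Each overlap writes the RespawnTransform component's world transform into SpawnTransform on BP_ThirdPersonGameMode.
; On the first overlap only, a DoOnce plays a timeline that rotates the flag arm, then plays a sound and spawns a Niagara burst above the respawn point.
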(event OnComponentBeginOverlap(Box)
  (params (OverlappedComponent :type Primitive%20Component%20Object%20Reference) (OtherActor :type Actor%20Object%20Reference) (OtherComp :type Primitive%20Component%20Object%20Reference) (OtherBodyIndex :type Integer) (bFromSweep :type Boolean) (SweepResult :type Hit%20Result%20Structure%20%28by%20ref%29))
  (Utilities|Casting|CastToBP_ThirdPersonCharacter OtherActor)
  (bind _asbp_third_person_game_mode (Utilities|Casting|CastToBP_ThirdPersonGameMode (Game|GetGameMode)))
  (Variables|/Game/ThirdPerson/Blueprints/BP_ThirdPersonGameMode.BP_ThirdPersonGameMode_C|SetSpawnTransform _asbp_third_person_game_mode (Transformation|GetWorldTransform (Variables|Default|GetRespawnTransform)))
  (Utilities|FlowControl|DoOnce false
    (:Completed
      (bind _flagalphaovertime (Timeline|RotateFlag PlayFromStart)
        (:Update
          (Transformation|SetRelativeRotation (Variables|Default|GetFlagArm) (Math|Rotator|Lerp(Rotator) (Variables|Default|GetFlagArmRotateStart) (Variables|Default|GetFlagArmRotateEnd) _flagalphaovertime) false false))
        (:Finished
          ;[0 0 0] SFX & VFX
          (Audio|PlaySound2D "/Engine/VREditor/Sounds/UI/Enter_Simulate.Enter_Simulate" 1.0 1.0 0.0 0 0)
          (Niagara|SpawnSystematLocation "/Niagara/DefaultAssets/Templates/Systems/RadialBurst.RadialBurst" (+ (Transformation|GetWorldLocation (Variables|Default|GetRespawnTransform)) "0.000000,0.000000,200.000000") "0, 0, 0" "10.000000,10.000000,10.000000"))))))

(event EventBeginPlay)

(event Collision|EventActorBeginOverlap
  (params (OtherActor :type Actor%20Object%20Reference)))

(event EventTick
  (params (DeltaSeconds :type Float%20%28single-precision%29)))

(fn ConstructionScript)