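; BP_Block_Breakable is a platformer block that breaks when hit and awards points.
; Its HitBlock event plays the interaction sound and particle effect slightly above the block, then spawns a BP_Points actor carrying the block's point value.
; It also adds those points through the player controller, then destroys itself.
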(event EventBeginPlay
  (|CallParentFunction) ; This node is disabled and will not be called.\nDrag off pins to build functionality.
)

(event EventHitBlock
  (bind _points (Variables|Default|GetPoints))
  (Utilities|FlowControl|Sequence
    (:then_0
      (CallFunction|PlayBlockInteractFX (Variables|Default|GetInteractSFX) 0 (Variables|Default|GetInteractVFX%28Particle%29) (+ (Transformation|GetActorLocation) "0.000000,0.000000,50.000000")))
    (:then_1
      (Game|SpawnActorfromClass "/Game/Platformer/Blueprints/BP_Points.BP_Points_C" (Transformation|GetActorTransform) "Undefined" "MultiplyWithRoot" 0 _points 0)
      (Default|AddPoints (Variables|Default|GetPlayerControler) _points))
    (:then_2
      (Actor|DestroyActor))))

(fn ConstructionScript
  (|CallParentFunction))