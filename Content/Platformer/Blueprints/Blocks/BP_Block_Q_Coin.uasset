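; A question-mark coin block for a platformer that rewards the player when HitBlock is called.
; The first hit plays interact effects, swaps the cube material, spawns points and coin actors, and credits both to the player controller.
; A timeline bumps the cube vertically, then the block is marked finished.
; Later hits only play a bump sound, throttled by a DoOnce that resets after a short delay.
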(event EventBeginPlay
  (|CallParentFunction) ; This node is disabled and will not be called.\nDrag off pins to build functionality.
)

(event EventHitBlock
  (bind _points (Variables|Default|GetPoints))
  (if (Variables|Default|GetfinishedInteracting)
    (Utilities|FlowControl|DoOnce true :!label _label
      (:Completed
        (Audio|PlaySound2D "/Game/Platformer/Audio/Mario_BrickBump.Mario_BrickBump" 1.0 1.0 0.0 0 0)
        (Utilities|FlowControl|Delay 0.5)
        (goto _label Reset)))
    (else
      (Utilities|FlowControl|Sequence
        (:then_0
          ;[0 0 0] 0) Play FX
          (CallFunction|PlayBlockInteractFX (Variables|Default|GetInteractSFX) 0 (Variables|Default|GetInteractVFX%28Particle%29) (+ (Transformation|GetActorLocation) "0.000000,0.000000,50.000000"))
          (Rendering|Material|SetMaterial (Variables|Default|GetCube) 0 (Variables|Default|GetInteractMaterial)))
        (:then_1
          ;[0.005208 0.005208 0.005208] 1) Add Points
          (Game|SpawnActorfromClass "/Game/Platformer/Blueprints/BP_Points.BP_Points_C" (Transformation|GetActorTransform) "Undefined" "MultiplyWithRoot" 0 _points 0)
          (Default|AddPoints (Variables|Default|GetPlayerControler) _points))
        (:then_2
          ;[0 0 0] 2) Add Coins
          (Game|SpawnActorfromClass "/Game/Platformer/Blueprints/Blocks/BP_Block_Coin.BP_Block_Coin_C" (Transformation|GetActorTransform) "Undefined" "MultiplyWithRoot" 0 0)
          (Default|AddCoins (Variables|Default|GetPlayerControler) (Variables|Default|GetCoinsToAdd)))
        (:then_3
          ;[0 0 0] 4) Block Animation
          (bind _movement (Timeline|BlockAim PlayFromStart)
            (:Update
              (Transformation|SetRelativeLocation (Variables|Default|GetCube) (Math|Vector|MakeVector 0.0 0.0 _movement) false false))))
        (:then_4
          (Variables|Default|SetfinishedInteracting true)
          (Utilities|FlowControl|Delay 0.5)
          (goto _label Reset))))))

(fn ConstructionScript
  (|CallParentFunction))