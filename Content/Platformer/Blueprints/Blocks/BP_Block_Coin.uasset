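; Coin effect actor, likely popped from a block, that plays a short animation and removes itself.
; On BeginPlay a timeline drives the Coin component's relative height and yaw, moving and rotating it.
; When the timeline finishes, it spawns the loot pickup particle at the coin's world location and destroys the actor.
; The file contains no overlap or scoring logic, so the actor is purely visual here.
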(event EventBeginPlay
  (Components|Timeline|SetPlayRate (Variables|Default|GetCoinAnimTimeline) 1.0)
  (bind (_direction _movement _rotation) (Timeline|CoinAnimTimeline PlayFromStart)
    (:Update
      (Transformation|SetRelativeLocationAndRotation (Variables|Default|GetCoin) (Math|Vector|MakeVector 0.0 0.0 _movement) (Math|Rotator|MakeRotator -7e+01 -9e+01 _rotation) false false))
    (:Finished
      (Effects|SpawnEmitteratLocation "/Game/InfinityBladeEffects/Effects/FX_Treasure/Loot/P_Loot_Pickup.P_Loot_Pickup" (Transformation|GetWorldLocation (Variables|Default|GetCoin)))
      (Actor|DestroyActor))))

(event Collision|EventActorBeginOverlap
  (params (OtherActor :type Actor%20Object%20Reference)))

(event EventTick
  (params (DeltaSeconds :type Float%20%28single-precision%29)))

(fn ConstructionScript)