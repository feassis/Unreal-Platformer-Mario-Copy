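; Base Blueprint for platformer blocks that react when the player character bumps them from below.
; On BeginPlay it casts and caches the first player controller as BP_PlayerController.
; The Cube's hit event calls HitBlock only for the player character with an impact normal Z of exactly one.
; HitBlock's behavior is not defined in these graphs.
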(event OnComponentHit(Cube)
  (params (HitComponent :type Primitive%20Component%20Object%20Reference) (OtherActor :type Actor%20Object%20Reference) (OtherComp :type Primitive%20Component%20Object%20Reference) (NormalImpulse :type Vector :default "0, 0, 0") (Hit :type Hit%20Result%20Structure%20%28by%20ref%29))
  (if (and (== OtherActor (Game|GetPlayerCharacter 0)) (== (.Z (Math|Vector|BreakVector (.ImpactNormal (Collision|BreakHitResult Hit)))) 1.0))
    (CallFunction|HitBlock)))

(event EventBeginPlay
  ;[0 0 0] Ref To Plkayer Controller
  (bind _asbp_player_controller (Utilities|Casting|CastToBP_PlayerController (Game|GetPlayerController 0)))
  (Variables|Default|SetPlayerControler _asbp_player_controller))

(fn ConstructionScript)