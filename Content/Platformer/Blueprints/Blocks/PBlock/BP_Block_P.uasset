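; Mario-style P-Block switch that the player stomps to temporarily toggle tagged blocks in a platformer level.
; A downward-normal hit from the player on the Box launches them upward, plays smash effects, music, camera shake and rumble, and swaps in the smashed meshes.
; It calls PBlockOn on tagged BP_Block_Base actors, then a timer calls PBlockOff on them and stops the music.
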(event OnComponentHit(Box)
  (params (HitComponent :type Primitive%20Component%20Object%20Reference) (OtherActor :type Actor%20Object%20Reference) (OtherComp :type Primitive%20Component%20Object%20Reference) (NormalImpulse :type Vector :default "0, 0, 0") (Hit :type Hit%20Result%20Structure%20%28by%20ref%29))
  (bind _returnvalue (Game|GetPlayerCharacter 0))
  (if (and (== OtherActor _returnvalue) (Utilities|Operators|EqualEqual (.ImpactNormal (Collision|BreakHitResult Hit)) "0.000000,0.000000,-1.000000" 0.01))
    (Character|LaunchCharacter _returnvalue "0.000000,0.000000,400.000000" false false)
    (Utilities|FlowControl|Sequence
      (:then_0
        ;[0 0 0] P_Block FX
        (Audio|PlaySound2D "/Game/Platformer/Audio/Mario_Thwomp.Mario_Thwomp" 1.0 1.0 0.0 0 0)
        (Effects|SpawnEmitteratLocation "/Game/InfinityBladeEffects/Effects/FX_Breakables/pot/P_PotBreak_Ceramic.P_PotBreak_Ceramic" (Transformation|GetWorldLocation (Variables|Default|GetBlock_P_Smashed)))
        (Audio|Components|Audio|Play (Variables|Default|GetMusic) 0.0))
      (:then_1
        ;[0 0 0] Camera Shake and Force Feedback
        (Camera|PlayWorldCameraShake "/Game/Platformer/Blueprints/Blocks/PBlock/BP_CamertaShake.BP_CamertaShake_C" (Transformation|GetActorLocation (Game|GetPlayerCharacter 0)) 1e+03 2e+03)
        (Game|Feedback|ClientPlayForceFeedback (Game|GetPlayerController 0) "/Game/Platformer/Blueprints/Blocks/PBlock/ForceFeedback.ForceFeedback" "None" false false false))
      (:then_2
        ;[0 0 0] Show Meshes $ Destrou Components
        (Rendering|SetVisibility (Variables|Default|GetBlock_P_Smashed) true false)
        (Components|DestroyComponent (Variables|Default|GetBox)))
      (:then_3
        ;[0 0 0] Find All Actors with PBlock Tag and Turn on function
        (bind _outactors (Actor|GetAllActorswithTag (Variables|Default|GetTag)))
        (bind _output_get (Variables|Default|SetBlocks _outactors))
        (for _array_element _output_get
          (bind _asbp_block_base (Utilities|Casting|CastToBP_Block_Base _array_element))
          (Default|PBlockon _asbp_block_base)))
      (:then_4
        ;[0 0 0] PBkock Timer
        (Utilities|Time|SetTimerbyEvent (delegate Custom|PBlockTimeOver) (Variables|Default|GetPBlockTimeDuration))))))

(event Custom|PBlockTimeOver
  ;[0 0 0] PBkock Timer
  (for _array_element (Variables|Default|GetBlocks)
    (bind _asbp_block_base (Utilities|Casting|CastToBP_Block_Base _array_element))
    (Default|PBlockOff _asbp_block_base))
  (Audio|Components|Audio|Stop (Variables|Default|GetMusic)))

(event EventBeginPlay)

(event Collision|EventActorBeginOverlap
  (params (OtherActor :type Actor%20Object%20Reference)))

(event EventTick
  (params (DeltaSeconds :type Float%20%28single-precision%29)))

(fn ConstructionScript)