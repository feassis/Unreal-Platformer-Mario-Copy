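; Platformer fire flower block that releases a power-up when hit and awards points on pickup.
; The first HitBlock plays effects, swaps the cube material and runs timelines to bump the block and move the flower, adding a glow afterwards.
; Later hits only play a bump sound, throttled by a delayed DoOnce reset.
; Player overlap with the flower box grants flower power, spawns a points actor, updates score and destroys the flower components.
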(event OnComponentBeginOverlap(Box_Flower)
  (params (OverlappedComponent :type Primitive%20Component%20Object%20Reference) (OtherActor :type Actor%20Object%20Reference) (OtherComp :type Primitive%20Component%20Object%20Reference) (OtherBodyIndex :type Integer) (bFromSweep :type Boolean) (SweepResult :type Hit%20Result%20Structure%20%28by%20ref%29))
  (bind _points (Variables|Default|GetPoints))
  (bind _asbp_third_person_character (Utilities|Casting|CastToBP_ThirdPersonCharacter OtherActor))
  (Default|GotFlowerPower _asbp_third_person_character)
  (Utilities|FlowControl|Sequence
    (:then_0
      ;[0.005208 0.005208 0.005208] 0) Add Points
      (Game|SpawnActorfromClass "/Game/Platformer/Blueprints/BP_Points.BP_Points_C" (Transformation|GetWorldTransform (Variables|Default|GetArrow)) "Undefined" "MultiplyWithRoot" 0 _points 0)
      (Default|AddPoints (Variables|Default|GetPlayerControler) _points))
    (:then_1
      ;[0 0 0] Destroy Block Components
      (Components|DestroyComponent (Variables|Default|GetBox_Flower)))))

(event EventBeginPlay
  (|CallParentFunction) ; This node is disabled and will not be called.\nDrag off pins to build functionality.
)

(event EventHitBlock
  (if (Variables|Default|GetfinishedInteracting)
    (Utilities|FlowControl|DoOnce true :!label _label
      (:Completed
        (Audio|PlaySound2D "/Game/Platformer/Audio/Mario_BrickBump.Mario_BrickBump" 1.0 1.0 0.0 0 0)
        (Utilities|FlowControl|Delay 0.5)
        (goto _label Reset)))
    (else
      (Utilities|FlowControl|Sequence
        (:then_0
          ;[0 0 0] 0) Play FX
          (CallFunction|PlayBlockInteractFX (Variables|Default|GetInteractSFX) 0 (Variables|Default|GetInteractVFX%28Particle%29) (+ (Transformation|GetActorLocation) "0.000000,0.000000,50.000000"))
          (Rendering|Material|SetMaterial (Variables|Default|GetCube) 0 (Variables|Default|GetInteractMaterial)))
        (:then_1
          ;[0 0 0] 1) Block Animation
          (bind _movement (Timeline|BlockAim PlayFromStart)
            (:Update
              (Transformation|SetRelativeLocation (Variables|Default|GetCube) (Math|Vector|MakeVector 0.0 0.0 _movement) false false))
            (:Finished
              (bind _returnvalue (Effects|SpawnEmitteratLocation "/Game/InfinityBladeEffects/Effects/FX_Treasure/Gold_Bag/P_DeadMans_Loot.P_DeadMans_Loot" (Transformation|GetWorldLocation (Variables|Default|GetFlower))))
              (Variables|Default|SetPowerUpGlow _returnvalue))))
        (:then_2
          ;[0 0 0] Flower Anim
          (bind _movement_2 (Timeline|FlowerAnim PlayFromStart)
            (:Update
              (bind _box_flower (Variables|Default|GetBox_Flower)
                (:then
                  (Transformation|SetRelativeLocation _box_flower (Math|Vector|MakeVector 0.0 0.0 _movement_2) false false))
                (:else)))))
        (:then_4
          (Variables|Default|SetfinishedInteracting true)
          (Utilities|FlowControl|Delay 0.5)
          (goto _label Reset))))))

(fn ConstructionScript
  (|CallParentFunction))