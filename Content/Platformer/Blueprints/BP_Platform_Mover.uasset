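; BP_Platform_Mover is a moving platform actor for a platformer level.
; On BeginPlay it sets the PlatformMovement timeline to a configurable PlayRate and plays it.
; Each timeline update moves the Platform component's relative location by lerping between LocStart and LocEnd using the Movement track, without sweep.
; The construction script, overlap and tick events add no logic.
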(event EventBeginPlay
  (|CallParentFunction)
  (Components|Timeline|SetPlayRate (Variables|Default|GetPlatformMovement) (Variables|Default|GetPlayRate))
  (bind _movement (Timeline|PlatformMovement Play)
    (:Update
      (Transformation|SetRelativeLocation (Variables|Default|GetPlatform) (Math|Vector|Lerp(Vector) (Variables|Default|GetLoc_Start) (Variables|Default|GetLoc_End) _movement) false false))))

(event Collision|EventActorBeginOverlap
  (params (OtherActor :type Actor%20Object%20Reference))
  (|CallParentFunction OtherActor) ; This node is disabled and will not be called.\nDrag off pins to build functionality.
)

(event EventTick
  (params (DeltaSeconds :type Float%20%28single-precision%29))
  (|CallParentFunction DeltaSeconds) ; This node is disabled and will not be called.\nDrag off pins to build functionality.
)

(fn ConstructionScript
  (|CallParentFunction))