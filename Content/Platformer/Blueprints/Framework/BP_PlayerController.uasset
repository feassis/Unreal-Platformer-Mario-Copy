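; Player controller for a platformer that tracks the player's coins and lives and shows the HUD.
; AddCoins adds to the coin count and, at 100 or more, grants a life, carries the remainder over, plays a 1-up sound and prints the total.
; BeginPlay creates the WBP_HUD widget and adds it to the viewport.
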(event Custom|AddCoins
  (params (CoinsToAdd :type Integer))
  ;[0 0.004675 0.02083] Add Coins
  (if (>= (+ CoinsToAdd (Variables|Default|GetCoins)) 100)
    (Variables|Default|SetLives (+ (Variables|Default|GetLives) 1))
    (Variables|Default|SetCoins (Math|Integer|Clamp(Integer) (- (+ CoinsToAdd (Variables|Default|GetCoins)) 100) 0 100))
    (Audio|PlaySound2D "/Game/Platformer/Audio/Mario_1up.Mario_1up" 1.0 1.0 0.0 0 0)
    (else
      (Variables|Default|SetCoins (Math|Integer|Clamp(Integer) (+ CoinsToAdd (Variables|Default|GetCoins)) 0 100))))
  (Development|PrintString (Utilities|String|Append "Coins" (Utilities|String|ToString(Integer) (Variables|Default|GetCoins)))))

(event EventTick
  (params (DeltaSeconds :type Float%20%28single-precision%29)))

(event EventBeginPlay
  ;[0 0 0] Add Hud To view port
  (bind _returnvalue (UserInterface|CreateWidget "/Game/Platformer/UI/WBP_HUD.WBP_HUD_C"))
  (UserInterface|Viewport|AddtoViewport _returnvalue 0))

(fn ConstructionScript)