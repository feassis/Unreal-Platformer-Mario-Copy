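; End-of-level flagpole actor that plays a Mario-style finish sequence when the player overlaps its trigger.
; It disables input, calls LevelComplete, then snaps the flag to the player's grab height, capped at its start.
; MoveComponentTo slides player and flag down before the player hops off and explodes.
; If the timer's last digit matches FireworkShowSpecialNumber, a self-calling DoN event spawns that many point-awarding fireworks at random points in a box.
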(event OnComponentBeginOverlap(TriggerVolume)
  (params (OverlappedComponent :type Primitive%20Component%20Object%20Reference) (OtherActor :type Actor%20Object%20Reference) (OtherComp :type Primitive%20Component%20Object%20Reference) (OtherBodyIndex :type Integer) (bFromSweep :type Boolean) (SweepResult :type Hit%20Result%20Structure%20%28by%20ref%29))
  (bind _playerendpoint (Variables|Default|GetPlayerEndPoint))
  (bind _flagendpoint (Variables|Default|GetFlagEndPoint))
  (bind _flag (Variables|Default|GetFlag))
  (bind _playerexplodepoint (Variables|Default|GetPlayerExplodePoint))
  (bind _flag_2 (Variables|Default|GetFlag))
  (bind _fireworksarea (Variables|Default|GetFireworksArea))
  (bind _returnvalue (Transformation|GetWorldLocation _flag))
  (bind (_x _y _z) (Math|Vector|BreakVector _returnvalue))
  ;[0 0 0] DetectPlayer Overlaping Fla pole trigger volume and disable input and calling LevelComplete Event
  (bind _asbp_third_person_character (Utilities|Casting|CastToBP_ThirdPersonCharacter OtherActor))
  (bind _output_get (Variables|Default|SetMyCharacter _asbp_third_person_character))
  (Input|DisableInput _output_get (Game|GetPlayerController 0))
  (Utilities|FlowControl|DoOnce false
    (:Completed
      (Default|CallLevelComplete)
      ;[0 0 0] Move Flag to locale where player cresssed trigger volume
      (if (> (.Z (Math|Vector|BreakVector (Transformation|GetWorldLocation (Variables|/Game/ThirdPerson/Blueprints/BP_ThirdPersonCharacter.BP_ThirdPersonCharacter_C|GetFlagAttachPoint (Variables|Default|GetMyCharacter))))) _z)
        (bind _output_get_2 (Variables|Default|SetFlagStartPoint (Math|Vector|MakeVector _x _y _z)))
        (Transformation|SetWorldLocation _flag_2 _output_get_2 false false)
        ;[0 0 0] Set player local when jumped over flag
        (Transformation|SetWorldLocation (Variables|/Script/Engine.Character|GetCapsuleComponent (Variables|Default|GetMyCharacter)) (Transformation|GetWorldLocation (Variables|Default|GetPlayerStartPoint)) false false)
        (else
          (bind _output_get_3 (Variables|Default|SetFlagStartPoint (Math|Vector|MakeVector _x _y (.Z (Math|Vector|BreakVector (Transformation|GetWorldLocation (Variables|/Game/ThirdPerson/Blueprints/BP_ThirdPersonCharacter.BP_ThirdPersonCharacter_C|GetFlagAttachPoint (Variables|Default|GetMyCharacter))))))))
          (Transformation|SetWorldLocation _flag_2 _output_get_3 false false)))
      ;[0 0 0] SetCharacter Position and Play Anim
      (Transformation|SetWorldRotation (Variables|/Script/Engine.Character|GetCapsuleComponent (Variables|Default|GetMyCharacter)) (Transformation|GetWorldRotation (Variables|Default|GetPlayerEndPoint)) false false)
      (Transformation|AddLocalOffset (Variables|/Script/Engine.Character|GetCapsuleComponent (Variables|Default|GetMyCharacter)) "0.000000,30.000000,0.000000" false false)
      (Variables|/Script/Engine.CharacterMovementComponent|SetGravityScale (Variables|/Script/Engine.Character|GetCharacterMovement (Variables|Default|GetMyCharacter)) 0.0)
      (Components|Activation|Deactivate (Variables|/Script/Engine.Character|GetCharacterMovement (Variables|Default|GetMyCharacter)))
      (Components|Animation|PlayAnimation (Variables|/Script/Engine.Character|GetMesh (Variables|Default|GetMyCharacter)) "/Game/Characters/Mannequins/Animations/Manny/MM_Run_Fwd.MM_Run_Fwd" false)
      (Components|Animation|SetPosition (Variables|/Script/Engine.Character|GetMesh (Variables|Default|GetMyCharacter)) 1.9 true)
      ;[0 0 0] Pause Before Playing SFX and Move Down The Pole
      (Utilities|FlowControl|Delay 1.0)
      (Audio|PlaySound2D "/Game/Platformer/Audio/Mario_FlagPole.Mario_FlagPole" 1.0 1.0 0.0 0 0)
      (Utilities|FlowControl|Sequence
        (:then_0
          ;[0 0 0] Animate Character down the pole
          (Components|MoveComponentTo (Variables|/Script/Engine.Character|GetCapsuleComponent (Variables|Default|GetMyCharacter)) (Transformation|GetWorldLocation _playerendpoint) (Transformation|GetWorldRotation _playerendpoint) false false 1.0 false)
          ;[0 0 0] Player At botton of Flag pole script
          (Components|Animation|PlayAnimation (Variables|/Script/Engine.Character|GetMesh (Variables|Default|GetMyCharacter)) "/Game/Characters/Mannequins/Animations/Manny/MM_Jump.MM_Jump" false)
          (Utilities|FlowControl|Delay 0.3)
          ;[0 0 0] Player Jump Of Flag Pole
          (Components|Animation|PlayAnimation (Variables|/Script/Engine.Character|GetMesh (Variables|Default|GetMyCharacter)) "/Game/Characters/Mannequins/Animations/Manny/MM_Fall_Loop.MM_Fall_Loop" false)
          (Components|MoveComponentTo (Variables|/Script/Engine.Character|GetCapsuleComponent (Variables|Default|GetMyCharacter)) (Transformation|GetWorldLocation _playerexplodepoint) (Transformation|GetWorldRotation _playerexplodepoint) false false 0.5 false)
          ;[0 0 0] Explode Player Script
          (Effects|SpawnEmitteratLocation "/Game/StarterContent/Particles/P_Explosion.P_Explosion" (Transformation|GetWorldLocation (Variables|/Script/Engine.Character|GetCapsuleComponent (Variables|Default|GetMyCharacter))) "0, 0, 0" "2.000000,2.000000,2.000000")
          (Audio|PlaySoundatLocation "/Game/StarterContent/Audio/Explosion_Cue.Explosion_Cue" (Transformation|GetWorldLocation (Variables|/Script/Engine.Character|GetCapsuleComponent (Variables|Default|GetMyCharacter))) "0, 0, 0" 1.0 1.0 0.0 0 0 0 0)
          (Rendering|SetVisibility (Variables|/Script/Engine.Character|GetCapsuleComponent (Variables|Default|GetMyCharacter)) false true)
          ;[0 0 0] Check if last digit of time remainig = to Fireshow number
          (if (== (Variables|Default|GetFireworkShowSpecialNumber) (Utilities|String|Right (Utilities|String|ToString(Integer) (Variables|/Game/Platformer/Blueprints/Framework/BP_PlayerController.BP_PlayerController_C|GetTimer (Variables|Default|GetMyControler))) 1))
            ;[0 0 0] Play Fire works and award player extra points
            (Utilities|FlowControl|Delay 0.5)
            (Utilities|FlowControl|DoN (Variables|Default|GetFireworkShowSpecialNumber)
              (:Exit
                (bind _output_get_4 (Variables|Default|SetFireworkLocale (Math|Random|RandomPointinBoundingBox (Transformation|GetWorldLocation _fireworksarea) (Variables|/Script/Engine.BoxComponent|GetBoxExtent _fireworksarea))))
                (Effects|SpawnEmitteratLocation "/Game/InfinityBladeEffects/Effects/FX_Monsters/FX_Monster_GolemBot/Notifies/P_SparkBurst.P_SparkBurst" _output_get_4 "0, 0, 0" "10.000000,10.000000,10.000000")
                (Audio|PlaySoundatLocation "/Game/Platformer/Audio/Mario_Thwomp.Mario_Thwomp" (Variables|Default|GetFireworkLocale) "0, 0, 0" 1.0 1.0 0.0 0 0 0 0)
                (Game|SpawnActorfromClass "/Game/Platformer/Blueprints/BP_Points.BP_Points_C" (Math|Transform|MakeTransform (Variables|Default|GetFireworkLocale)) "Undefined" "MultiplyWithRoot" 0 (Variables|Default|GetFireworkPoints) 0)
                (Default|AddPoints (Variables|Default|GetMyControler) (Variables|Default|GetFireworkPoints))
                (CallFunction|MoreFireworkds)))))
        (:then_1
          ;[0 0 0] Animate Flag Down The Pole
          (Components|MoveComponentTo (Variables|Default|GetFlag) (Variables|/Script/Engine.SceneComponent|GetRelativeLocation _flagendpoint) (Variables|/Script/Engine.SceneComponent|GetRelativeRotation _flagendpoint) false false 1.0 false))))))

(event Custom|More%20Fireworkds
  (bind _fireworksarea (Variables|Default|GetFireworksArea))
  ;[0 0 0] Play Fire works and award player extra points
  (Utilities|FlowControl|Delay 0.5)
  (Utilities|FlowControl|DoN (Variables|Default|GetFireworkShowSpecialNumber)
    (:Exit
      (bind _output_get (Variables|Default|SetFireworkLocale (Math|Random|RandomPointinBoundingBox (Transformation|GetWorldLocation _fireworksarea) (Variables|/Script/Engine.BoxComponent|GetBoxExtent _fireworksarea))))
      (Effects|SpawnEmitteratLocation "/Game/InfinityBladeEffects/Effects/FX_Monsters/FX_Monster_GolemBot/Notifies/P_SparkBurst.P_SparkBurst" _output_get "0, 0, 0" "10.000000,10.000000,10.000000")
      (Audio|PlaySoundatLocation "/Game/Platformer/Audio/Mario_Thwomp.Mario_Thwomp" (Variables|Default|GetFireworkLocale) "0, 0, 0" 1.0 1.0 0.0 0 0 0 0)
      (Game|SpawnActorfromClass "/Game/Platformer/Blueprints/BP_Points.BP_Points_C" (Math|Transform|MakeTransform (Variables|Default|GetFireworkLocale)) "Undefined" "MultiplyWithRoot" 0 (Variables|Default|GetFireworkPoints) 0)
      (Default|AddPoints (Variables|Default|GetMyControler) (Variables|Default|GetFireworkPoints))
      (CallFunction|MoreFireworkds))))

(event EventBeginPlay
  ;[0 0 0] Ref to Player Controller
  (bind _asbp_player_controller (Utilities|Casting|CastToBP_PlayerController (Game|GetPlayerController 0)))
  (Variables|Default|SetMyControler _asbp_player_controller))

(fn ConstructionScript)